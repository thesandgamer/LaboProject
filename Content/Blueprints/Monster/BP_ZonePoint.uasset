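; Monster zone helper that finds a spawn location around the most attractive takable object in the level.
; GetObjects has every BP_P_Takable evaluate its surroundings within a radius and keeps the highest non-zero total attraction.
; If that meets the minimum, FindPosToSpawn retries random points until one lies in the ring between inner and outer radius and a vertical trace hits.
; Debug circles, traces and prints show the search, and CalculateScoreAttirance is empty.
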(fn `CalculateScoreAttirance`)

(fn `FindPosToSpawn`
  (params (MinValueToDetect :type "Float (double-precision)"))
  (returns (Location :type "Vector Structure") (Object :type "/Game/Blueprints/Objects/BP_P_Takable Object Reference") (FindSomething :type Boolean))
  (locals (AreNotFindLocation :type Boolean :default true) (LocationToSpawn :type "Vector Structure" :default (0.0 0.0 0.0)))
  (bind (_object _valuemaximum) (`self.GetObjects`))
  (`/Engine/EditorBlueprintResources/StandardMacros.IsValid` _object
    (:`Is Valid`
      (if (>= _valuemaximum MinValueToDetect)
        (bind _returnvalue (`self.K2_GetActorLocation` _object))
        (`KismetSystemLibrary.DrawDebugCircle` _returnvalue (`self.OuterRadius`) 100 (struct :`R` 1.0 :`G` 1.0 :`B` 1.0 :`A` 1.0) 50.0 10.0 (0.0 1.0 0.0) (1.0 0.0 0.0))
        (`KismetSystemLibrary.DrawDebugCircle` _returnvalue (`self.InnerRadius`) 100 (struct :`R` 1.0 :`G` 1.0 :`B` 1.0 :`A` 1.0) 50.0 10.0 (0.0 1.0 0.0) (1.0 0.0 0.0))
        (while (`local.AreNotFindLocation`)
          (bind (_location _completed) (`self.GetPositionOfSpawn` (`self.K2_GetActorLocation` _object)))
          (set `local.AreNotFindLocation` (not _completed))
          (set `local.LocationToSpawn` _location))
        (return (`local.LocationToSpawn`) _object true)
        (else
          (return (0.0 0.0 0.0) null false))))))

(fn `GetObjects`
  (returns (Object :type "/Game/Blueprints/Objects/BP_P_Takable Object Reference") (ValueMaximum :type "Float (double-precision)"))
  (locals (MaxAttirance :type "Float (double-precision)"))
  (bind _maxattirance (`local.MaxAttirance`))
  (set `self.MaxAttiranceObject` null)
  (set `local.MaxAttirance` 0.0)
  (set `self.MinValueToDetect` 0.0)
  (bind _outactors (`GameplayStatics.GetAllActorsOfClass` "/Game/Blueprints/Objects/BP_P_Takable.BP_P_Takable_C"))
  (for _array_element _outactors
    (`/Game/Blueprints/Objects/BP_P_Takable.GetAroundObjects` _array_element (`self.RadiusToDetectObjects`))
    (bind _totalattirancevalue (`/Game/Blueprints/Objects/BP_P_Takable.TotalAttiranceValue` _array_element))
    (if (!= _totalattirancevalue 0.0)
      (if (>= _totalattirancevalue (`local.MaxAttirance`))
        (set `local.MaxAttirance` _totalattirancevalue)
        (set `self.MaxAttiranceObject` _array_element))))
  (`KismetSystemLibrary.PrintString` (`KismetStringLibrary.Concat_StrStr` "Temp value " (`KismetStringLibrary.Conv_DoubleToString` _maxattirance)))
  (return (`self.MaxAttiranceObject`) _maxattirance))

(fn `GetPositionOfSpawn`
  (params (Origin :type "Vector Structure"))
  (returns (Location :type "Vector Structure") (Completed :type Boolean))
  (locals (RandomX :type "Float (double-precision)") (RandomY :type "Float (double-precision)") (InDonut :type Boolean) (LocationX :type "Float (double-precision)") (LocationY :type "Float (double-precision)"))
  (bind (_incircle _locationx _locationy) (`self.Is In Circle` (`self.OuterRadius`) Origin (`local.RandomX`) (`local.RandomY`)))
  (set `local.RandomX` (`KismetMathLibrary.RandomFloatInRange` (* (`self.OuterRadius`) -1.0) (`self.OuterRadius`)))
  (set `local.RandomY` (`KismetMathLibrary.RandomFloatInRange` (* (`self.OuterRadius`) -1.0) (`self.OuterRadius`)))
  (set `local.InDonut` (and _incircle (not (`self.Is In Circle` (`self.InnerRadius`) Origin (`local.RandomX`) (`local.RandomY`)))))
  (if (`local.InDonut`)
    (set `local.LocationX` _locationx)
    (set `local.LocationY` _locationy)
    (bind (_outhit _returnvalue) (`KismetSystemLibrary.LineTraceSingle` :`Start` (`KismetMathLibrary.MakeVector` (`local.LocationX`) (`local.LocationY`) 5000.0) :`End` (`KismetMathLibrary.MakeVector` (`local.LocationX`) (`local.LocationY`) -5000.0) :`TraceChannel` "TraceTypeQuery1" :`DrawDebugType` "ForDuration" :`TraceColor` (struct :`G` 0.005394 :`B` 1.0 :`A` 1.0) :`DrawTime` 50.0))
    (if _returnvalue
      (return (`.ImpactPoint` (`GameplayStatics.BreakHitResult` _outhit)) true)
      (else
        (return (0.0 0.0 0.0) false)))
    (else
      (return (0.0 0.0 0.0) false))))

(fn `Is In Circle`
  (params (Radius :type "Float (double-precision)") (CirclePos :type "Vector Structure") (PointToCheckX :type "Float (double-precision)") (PointToCheckY :type "Float (double-precision)"))
  (returns (InCircle :type Boolean) (LocationX :type "Float (double-precision)") (LocationY :type "Float (double-precision)"))
  (bind _returnvalue (+ (.x CirclePos) PointToCheckX))
  (bind _returnvalue_2 (+ (.y CirclePos) PointToCheckY))
  (bind (_returnvalue_x _returnvalue_y) (`KismetMathLibrary.BreakVector` (`KismetMathLibrary.MakeVector` _returnvalue _returnvalue_2)))
  (return (<= (+ (`KismetMathLibrary.Square` (- _returnvalue_x (.x CirclePos))) (`KismetMathLibrary.Square` (- _returnvalue_y (.y CirclePos)))) (`KismetMathLibrary.Square` Radius)) _returnvalue _returnvalue_2))

(fn `UserConstructionScript`)