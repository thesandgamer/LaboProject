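; Spawn zone actor that relocates the game's boss monster to its own sprite's location, provided the spot is clear.
; On BeginPlay a box overlap test checks for blocking objects; if none, ReplaceBoss teleports the monster below the sprite and disables its capsule collision.
; The Repositionne timeline then drives the monster's height, and on finish sets the MonsterAi state and destroys the zone.
; AI UnPossess/Possess nodes are left disconnected.
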(event `self.ReceiveBeginPlay`
  (bind _box (`self.Box`))
  (bind (_outactors _returnvalue) (`KismetSystemLibrary.ComponentOverlapActors` _box (`SceneComponent.K2_GetComponentToWorld` _box) (`|MakeArray` "ObjectTypeQuery1" "ObjectTypeQuery7" "ObjectTypeQuery2" :!type "EObjectTypeQuery Enum")))
  (set `self.ColliderOther` _returnvalue)
  (if (not _returnvalue)
    (`self.ReplaceBoss`)))

(event `ReplaceBoss`
  (bind (_returnvalue_x _returnvalue_y _returnvalue_z) (`KismetMathLibrary.BreakVector` (`SceneComponent.K2_GetComponentLocation` (`self.PaperSprite`))))
  (bind (_returnvalue_x_2 _returnvalue_y_2 _returnvalue_z_2) (`KismetMathLibrary.BreakVector` (`SceneComponent.K2_GetComponentLocation` (`self.PaperSprite`))))
  (bind _asgm_game (cast `/Game/Blueprints/A_Game/GM_Game` (`GameplayStatics.GetGameMode`) :!pure true))
  (bind _monster (`/Game/Blueprints/A_Game/GM_Game.Monster` _asgm_game))
  (`self.K2_SetActorLocation` _monster (`KismetMathLibrary.MakeVector` _returnvalue_x _returnvalue_y (- _returnvalue_z 500.0)) false true)
  (`PrimitiveComponent.SetCollisionEnabled` (`Character.CapsuleComponent` _monster) "NoCollision")
  (bind (_direction _value) (`Timeline|Repositionne`)
    (:`Update`
      (`self.K2_SetActorLocation` _monster (`KismetMathLibrary.MakeVector` _returnvalue_x_2 _returnvalue_y_2 (+ (- _returnvalue_z_2 400.0) (* _value 500.0))) false false))
    (:`Finished`
      (set `/Game/Blueprints/Monster/AI/AIC_Monster.State` "NewEnumerator1" (`/Game/Blueprints/A_Game/GM_Game.MonsterAi` _asgm_game))
      (`self.K2_DestroyActor`))))

(fn `UserConstructionScript`)