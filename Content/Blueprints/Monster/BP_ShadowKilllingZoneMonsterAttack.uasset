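; Monster attack actor that acts as an expanding killing zone for the dream player.
; Each tick it grows its radius by a fixed step, independent of delta time and uncapped, and sphere-traces for pawns, ignoring the game mode's Monster.
; A hit P_DreamPlayer gets Die called, possibly on repeated ticks, and the actor destroys itself after a short delay.
; The trace's debug sphere is drawn every frame.
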(event `self.ReceiveTick`
  (params (DeltaSeconds :type "Float (single-precision)"))
  (bind _returnvalue (`self.K2_GetActorLocation`))
  (set `self.Radius` (+ (`self.Radius`) 5.0))
  (bind (_outhit _returnvalue_2) (`KismetSystemLibrary.SphereTraceSingleForObjects` _returnvalue _returnvalue (`self.Radius`) (`|MakeArray` "ObjectTypeQuery3" :!type "EObjectTypeQuery Enum") false (`|MakeArray` (`/Game/Blueprints/A_Game/GM_Game.Monster` (cast `/Game/Blueprints/A_Game/GM_Game` (`GameplayStatics.GetGameMode`) :!pure true)) :!type "Actor Object Reference") "ForOneFrame"))
  (if _returnvalue_2
    (bind _asp_dream_player (cast `/Game/Blueprints/DreamPlayer/P_DreamPlayer` (`.HitActor` (`GameplayStatics.BreakHitResult` _outhit))))
    (`/Game/Blueprints/DreamPlayer/P_DreamPlayer.Die` _asp_dream_player)
    (`KismetSystemLibrary.Delay` 1.8)
    (`self.K2_DestroyActor`)))

(fn `UserConstructionScript`)