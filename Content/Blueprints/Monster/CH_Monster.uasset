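; Monster character Blueprint that gives an AI-controlled creature sight and a look-around behavior.
; While looking, a fast looping timer runs Look, which casts rings of debug-drawn line traces from Eyes toward SeeLocation.
; MoveLookLocation sweeps SeeLocation through Locations, then returns it to base and flags completion for LookAround.
; Spotting the player or a takable object halts looking and writes ActorSeen and PosToGo to the Blackboard.
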(event `self.ReceiveBeginPlay`
  ;[1 1 1] Comment
  (set `self.BaseLocationLooking` (`SceneComponent.RelativeLocation` (`self.SeeLocation`))))

(event `StartLooking`
  (bind _returnvalue (`KismetSystemLibrary.K2_SetTimer` self "Look" 0.01 true))
  (set `self.LookingTimer` _returnvalue))

(event `self.ReceiveTick`
  (params (DeltaSeconds :type "Float (single-precision)")))

(event `StopLooking`
  (`KismetSystemLibrary.K2_ClearAndInvalidateTimerHandle` (`self.LookingTimer`)))

(event `FindSomething`
  (bind _lookingpos (`self.LookingPos`))
  (`|ExecutionSequence`
    (:`then_0`
      (set `self.Find` true)
      (`KismetSystemLibrary.K2_ClearAndInvalidateTimerHandle` (`self.LookingTimer`)))
    (:`then_1`
      (goto _label :!via `Stop`))
    (:`then_2`
      (goto _label_2 :!via `Stop`))))

(event `MoveLookLocation`
  (bind _lookingpos (`self.LookingPos`))
  (set `self.FinishLookingAround` false)
  (`KismetSystemLibrary.MoveComponentTo` (`self.SeeLocation`) (`|GetArrayItem` (`self.Locations`) (`self.LookingPos`)) (struct) true true (`self.MoveLookTime`) :!label _label)
  (if (< _lookingpos (- (`KismetArrayLibrary.Array_Length` (`self.Locations`)) 1))
    (`/Engine/EditorBlueprintResources/StandardMacros.IncrementInt` _lookingpos
      (:`  `
        (`KismetSystemLibrary.Delay` 1.0)
        (goto _label)))
    (else
      (set `self.LookingPos` 0)
      (`KismetSystemLibrary.PrintString` "Finish looking")
      (if (not (`self.Find`))
        (`KismetSystemLibrary.MoveComponentTo` (`self.SeeLocation`) (`self.BaseLocationLooking`) (struct) true true (`self.MoveLookTime`) :!label _label_2)
        (set `self.FinishLookingAround` true)))))

(fn `Look`
  (bind _eyes (`self.Eyes`))
  (bind _numberoftrace (`self.NumberOfTrace`))
  (bind _returnvalue (`SceneComponent.K2_GetComponentLocation` _eyes))
  (bind _returnvalue_2 (`AIBlueprintHelperLibrary.GetBlackboard` (`AIBlueprintHelperLibrary.GetAIController` self)))
  (for _index (range (+ (`self.NumberIneTrace`) 1))
    (for _index_2 (range (+ _numberoftrace 1))
      (bind (_outhit _returnvalue_3) (`KismetSystemLibrary.LineTraceSingle` :`Start` _returnvalue :`End` (+ _returnvalue (`KismetMathLibrary.GreaterGreater_VectorRotator` (`KismetMathLibrary.GreaterGreater_VectorRotator` (+ (`SceneComponent.GetForwardVector` _eyes) (`KismetMathLibrary.MakeVector` (`self.Length`) (- (`self.Radius`) (`KismetMathLibrary.Conv_IntToDouble` (* (+ _index 1) 50))))) (`KismetMathLibrary.MakeRotator` (* _index_2 (/ 360.0 (`KismetMathLibrary.Conv_IntToDouble` (+ _numberoftrace 1)))))) (`KismetMathLibrary.FindLookAtRotation` (`SceneComponent.K2_GetComponentLocation` (`self.Eyes`)) (`SceneComponent.K2_GetComponentLocation` (`self.SeeLocation`))))) :`TraceChannel` "TraceTypeQuery1" :`DrawDebugType` "ForOneFrame" :`TraceHitColor` (struct :`R` 1.0 :`G` 1.0 :`B` 1.0 :`A` 1.0)))
      (if _returnvalue_3
        (bind (_bblockinghit _binitialoverlap _time _distance _location _impactpoint _normal _impactnormal _physmat _hitactor) (`GameplayStatics.BreakHitResult` _outhit))
        (bind _returnvalue_4 (`GameplayStatics.GetObjectClass` _hitactor))
        ;[1 1 1] Si joueur ou objet vu
        (if (or (== _returnvalue_4 "/Game/Blueprints/DreamPlayer/P_DreamPlayer.P_DreamPlayer_C") (== _returnvalue_4 "/Game/Blueprints/Objects/BP_P_Takable.BP_P_Takable_C"))
          (`KismetSystemLibrary.DrawDebugSphere` _impactpoint 10.0 12 (struct :`R` 0.950843 :`B` 1.0 :`A` 1.0))
          (`self.FindSomething`)
          (`BlackboardComponent.SetValueAsObject` _returnvalue_2 "ActorSeen" _hitactor)
          (`BlackboardComponent.SetValueAsVector` _returnvalue_2 "PosToGo" (`self.K2_GetActorLocation` _hitactor)))))))

(fn `LookAround`
  (returns (FinishLookingAround :type Boolean))
  (return (`self.FinishLookingAround`)))

(fn `UserConstructionScript`)