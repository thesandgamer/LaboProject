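; Bp_MonsterInReality is a monster stand-in whose skeletal mesh appears and disappears with the CH_Monster actor's looking state.
; On BeginPlay it hides the mesh, finds CH_Monster with GetActorOfClass and binds to its start and stop looking dispatchers.
; The start event shows the mesh and the stop event hides it, so visibility is event-driven with no Tick logic.
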(event `self.ReceiveBeginPlay`
  (`SceneComponent.SetVisibility` (`self.SkeletalMesh`) false false)
  (bind _returnvalue (`GameplayStatics.GetActorOfClass` "/Game/Blueprints/Monster/CH_Monster.CH_Monster_C"))
  (add `/Game/Blueprints/Monster/CH_Monster.ev_StartLooking` _returnvalue (delegate `Show`))
  (add `/Game/Blueprints/Monster/CH_Monster.Ev_StopLooking` _returnvalue (delegate `Hide`)))

(event `Show`
  (`SceneComponent.SetVisibility` (`self.SkeletalMesh`) true false))

(event `Hide`
  (`SceneComponent.SetVisibility` (`self.SkeletalMesh`) false false))

(fn `UserConstructionScript`)