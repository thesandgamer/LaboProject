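; Player controller that switches the player between a Reality world and a Dream world on the ChangeWorld input.
; Each switch blocking-loads the destination streamed level, unloads the other, has GM_Game set the pawns and possesses that world's pawn.
; Entering the dream calls RealityPawn's sleep and wake functions around the load; leaving releases any telekinesis-held actor.
; Key presses also track whether a gamepad is in use.
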(event `Key|AnyKey` :consume false
  (params (Key :type "Key Structure"))
  (:`Pressed`
    (set `self.UsingGamepad` (`KismetInputLibrary.Key_IsGamepadKey` Key))))

(event `PassIntoDream`
  (bind _realitypawn (`self.RealityPawn`))
  (set `self.InDream` true)
  (`/Game/Blueprints/RealityPlayer/P_RealityPlayer.Endormissement` _realitypawn)
  (`GameplayStatics.LoadStreamLevelBySoftObjectPtr` "/Game/Maps/Map_S_DreamMain.Map_S_DreamMain" true true)
  (`/Game/Blueprints/RealityPlayer/P_RealityPlayer.Reveil` _realitypawn)
  (`/Game/Blueprints/A_Game/GM_Game.SetPawns` (cast `/Game/Blueprints/A_Game/GM_Game` (`GameplayStatics.GetGameMode`) :!pure true))
  (`self.Possess` (`self.DreamPawn`))
  (`GameplayStatics.UnloadStreamLevelBySoftObjectPtr` "/Game/Maps/Map_S_Reality.Map_S_Reality" true))

(event `InputAction|ChangeWorld`
  (params (Key :type "Key Structure"))
  (:`Pressed`
    (if (`self.InDream`)
      (`self.PassIntoReality`)
      (else
        (`self.PassIntoDream`)))))

(event `PassIntoReality`
  (bind _dreampawn (`self.DreamPawn`))
  (set `self.InDream` false)
  (`GameplayStatics.LoadStreamLevelBySoftObjectPtr` "/Game/Maps/Map_S_Reality.Map_S_Reality" true true)
  (`/Engine/EditorBlueprintResources/StandardMacros.IsValid` (`/Game/Blueprints/DreamPlayer/P_DreamPlayer.ActorTaken` _dreampawn)
    (:`Is Valid`
      (`/Game/Blueprints/DreamPlayer/P_DreamPlayer.TelekinesisRelease` _dreampawn))
    (:`Is Not Valid`
      _))
  (`GameplayStatics.UnloadStreamLevelBySoftObjectPtr` "/Game/Maps/Map_S_DreamMain.Map_S_DreamMain" true)
  (`/Game/Blueprints/A_Game/GM_Game.SetPawns` (cast `/Game/Blueprints/A_Game/GM_Game` (`GameplayStatics.GetGameMode`) :!pure true))
  (`self.Possess` (`self.RealityPawn`)))

(fn `UserConstructionScript`)