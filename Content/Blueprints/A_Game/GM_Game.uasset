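; GM_Game is the game mode that wires up the player's dream and reality pawns when play begins.
; It finds the first P_DreamPlayer and P_RealityPlayer in the level and stores them on PC_Player.
; If the reality pawn is valid, the controller possesses it and then immediately calls PassIntoDream on PC_Player.
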(event `self.ReceiveBeginPlay`
  (bind _returnvalue (`GameplayStatics.GetPlayerController` 0))
  (bind _aspc_player (cast `/Game/Blueprints/A_Game/PC_Player` _returnvalue :!pure true))
  (bind _realitypawn (`/Game/Blueprints/A_Game/PC_Player.RealityPawn` _aspc_player))
  (`self.SetPawns`)
  (`/Engine/EditorBlueprintResources/StandardMacros.IsValid` _realitypawn
    (:`Is Valid`
      (`Controller.Possess` _returnvalue _realitypawn)
      (`/Game/Blueprints/A_Game/PC_Player.PassIntoDream` _aspc_player))))

(event `SetPawns`
  (bind _aspc_player (cast `/Game/Blueprints/A_Game/PC_Player` (`GameplayStatics.GetPlayerController` 0)))
  (bind _outactors (`GameplayStatics.GetAllActorsOfClass` "/Game/Blueprints/DreamPlayer/P_DreamPlayer.P_DreamPlayer_C"))
  (bind _outactors_2 (`GameplayStatics.GetAllActorsOfClass` "/Game/Blueprints/RealityPlayer/P_RealityPlayer.P_RealityPlayer_C"))
  (set `/Game/Blueprints/A_Game/PC_Player.DreamPawn` (`|GetArrayItem` _outactors) _aspc_player)
  (set `/Game/Blueprints/A_Game/PC_Player.RealityPawn` (`|GetArrayItem` _outactors_2) _aspc_player))

(fn `UserConstructionScript`)