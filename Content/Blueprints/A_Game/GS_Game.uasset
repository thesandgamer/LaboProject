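; GS_Game, apparently the GameState, handles passing objects into the dream world and respawning the player's DreamPawn.
; SpawnObject creates an actor of a given class and scale, flagged InDream, at an offset from the DreamPawn, then calls its feedback, BringReality and ResetRotation functions.
; Respawn moves the DreamPawn to CurrentSavePoint and destroys every BP_P_Takable actor.
; Both functions reach the pawn through PC_Player on player controller 0.
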(fn `Respawn`
  (`self.K2_SetActorLocation` (`/Game/Blueprints/A_Game/PC_Player.DreamPawn` (cast `/Game/Blueprints/A_Game/PC_Player` (`GameplayStatics.GetPlayerController` 0) :!pure true)) (`self.CurrentSavePoint`) false false)
  (bind _outactors (`GameplayStatics.GetAllActorsOfClass` "/Game/Blueprints/Objects/BP_P_Takable.BP_P_Takable_C"))
  (for _array_element _outactors
    (`self.K2_DestroyActor` _array_element)))

(fn `SpawnObject`
  (params (Class :type "/Game/Blueprints/Objects/BP_P_Takable Class Reference") (ScaleMultiplier :type "Float (double-precision)"))
  (bind _dreampawn (`/Game/Blueprints/A_Game/PC_Player.DreamPawn` (cast `/Game/Blueprints/A_Game/PC_Player` (`GameplayStatics.GetPlayerController` 0) :!pure true)))
  (bind (_returnvalue_x _returnvalue_y _returnvalue_z) (`KismetMathLibrary.BreakVector` (`SceneComponent.K2_GetComponentLocation` (`Character.CapsuleComponent` (`/Game/Blueprints/A_Game/PC_Player.DreamPawn` (cast `/Game/Blueprints/A_Game/PC_Player` (`GameplayStatics.GetPlayerController` 0) :!pure true))))))
  (bind _returnvalue (`|SpawnActorFromClass` Class (`KismetMathLibrary.MakeTransform` (`KismetMathLibrary.MakeVector` (+ _returnvalue_x 60.0) _returnvalue_y (+ _returnvalue_z 60.0)) (struct) (* (`KismetMathLibrary.Vector_One`) ScaleMultiplier)) "Undefined" "OverrideRootScale" null ScaleMultiplier true null))
  (`/Game/Blueprints/DreamPlayer/P_DreamPlayer.PassObjToAnotherWorldFeedback` _dreampawn)
  (`KismetSystemLibrary.PrintString` (`KismetSystemLibrary.GetClassDisplayName` Class))
  (`/Game/Blueprints/DreamPlayer/P_DreamPlayer.BringReality` _dreampawn _returnvalue)
  (`/Game/Blueprints/DreamPlayer/P_DreamPlayer.ResetRotation` _dreampawn))

(fn `UserConstructionScript`)