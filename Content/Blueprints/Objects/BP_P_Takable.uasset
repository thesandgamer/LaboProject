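; BP_P_Takable is a takable object that tracks box overlaps and measures the combined attraction of takables around it in the dream.
; Overlap events toggle IsColliding, while the Destroyed event spawns a Niagara pouf before removing the actor after a short delay.
; When InDream, GetAroundObjects sphere-traces, itself included, to fill ActorsNear and sum FacteurAttirance into TotalAttiranceValue, shown as debug text.
; Player-step detection, material swaps and marking neighbours as Calculé are disconnected.
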(event `self.ReceiveDestroyed`
  (`self.Destroyed`))

(event `self.Box.OnComponentBeginOverlap`
  (params (OverlappedComponent :type "PrimitiveComponent Object Reference") (OtherActor :type "Actor Object Reference") (OtherComp :type "PrimitiveComponent Object Reference") (OtherBodyIndex :type Integer) (bFromSweep :type Boolean) (SweepResult :type "HitResult Structure (by ref)"))
  (set `self.IsColliding` true))

(event `self.Box.OnComponentEndOverlap`
  (params (OverlappedComponent :type "PrimitiveComponent Object Reference") (OtherActor :type "Actor Object Reference") (OtherComp :type "PrimitiveComponent Object Reference") (OtherBodyIndex :type Integer))
  (set `self.IsColliding` false))

(event `RemoveActor`
  (`KismetSystemLibrary.Delay` 1.0)
  (`self.K2_DestroyActor`))

(fn `Destroyed`
  (`NiagaraFunctionLibrary.SpawnSystemAtLocation` "/Game/VFX/PlaceHolders/NS_Pouf.NS_Pouf" (`SceneComponent.K2_GetComponentLocation` (`self.Mesh`)) (struct) (2.0 2.0 2.0))
  (`self.RemoveActor`))

(fn `GetAroundObjects`
  (params (Radius :type "Float (double-precision)"))
  (bind (_returnvalue_x _returnvalue_y _returnvalue_z) (`KismetMathLibrary.BreakVector` (`self.K2_GetActorLocation`)))
  (bind _returnvalue (`self.K2_GetActorLocation`))
  (set `self.Calculé` false)
  (set `self.TotalAttiranceValue` 0.0)
  (`KismetArrayLibrary.Array_Clear` (`self.ActorsNear`))
  (if (`self.InDream`)
    (bind (_outhits _returnvalue_2) (`KismetSystemLibrary.SphereTraceMultiForObjects` :`Start` _returnvalue :`End` _returnvalue :`Radius` Radius :`ObjectTypes` (`|MakeArray` "ObjectTypeQuery7" :!type "EObjectTypeQuery Enum") :`DrawDebugType` "ForDuration" :`bIgnoreSelf` false))
    (if _returnvalue_2
      (for _array_element _outhits
        (bind _asbp_p_takable (cast `/Game/Blueprints/Objects/BP_P_Takable` (`.HitActor` (`GameplayStatics.BreakHitResult` _array_element))))
        (`|ExecutionSequence`
          (:`then_0`
            (`KismetArrayLibrary.Array_Add` (`self.ActorsNear`) _asbp_p_takable))
          (:`then_1`
            (if (not (`/Game/Blueprints/Objects/BP_P_Takable.Calculé` _asbp_p_takable))
              (set `self.TotalAttiranceValue` (+ (`self.TotalAttiranceValue`) (`/Game/Blueprints/Objects/BP_P_Takable.FacteurAttirance` _asbp_p_takable)))))))
      (`KismetSystemLibrary.DrawDebugString` (`KismetMathLibrary.MakeVector` _returnvalue_x _returnvalue_y (+ _returnvalue_z 500.0)) (`KismetStringLibrary.Conv_DoubleToString` (`self.TotalAttiranceValue`)) null (struct :`R` 1.0 :`B` 0.99368 :`A` 1.0) 20.0))))

(fn `UserConstructionScript`)