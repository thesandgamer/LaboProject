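; BP_FinalStair is an activable gameplay element, a stair that moves vertically when activated.
; It caches its actor location on BeginPlay, and its Activate override calls the parent and then the MonteLeTout event.
; That event prints a debug "Hello" and plays a timeline that lerps the actor's Z from the cached height to TargetZ, an absolute world height, keeping X and Y fixed.
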(event `self.ReceiveBeginPlay`
  (`parent.ReceiveBeginPlay`)
  (set `self.BaseLocation` (`self.K2_GetActorLocation`)))

(event `MonteLeTout`
  (bind (_baselocation_x _baselocation_y _baselocation_z) (`KismetMathLibrary.BreakVector` (`self.BaseLocation`)))
  (`KismetSystemLibrary.PrintString` "Hello")
  (bind (_direction _value) (`Timeline|Timeline_0`)
    (:`Update`
      (`self.K2_SetActorLocation` (`KismetMathLibrary.MakeVector` _baselocation_x _baselocation_y (`KismetMathLibrary.Lerp` _baselocation_z (`self.TargetZ`) _value))))))

(fn `Activate`
  (`parent.Activate`)
  (`self.MonteLeTout`))

(fn `UserConstructionScript`
  (`parent.UserConstructionScript`))