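; BP_Door is an activable gameplay element that swings a door open by rotating its pivot component.
; It overrides Activate and DeActivate, calling the parent version and then playing or reversing the RotationDoor timeline.
; The timeline value scales a configurable RotationAxis to set the relative rotation of RotPoint.
; Reversal on deactivation happens only when OpenClose is true, so otherwise the door stays open.
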(event `Rotate`
  (bind (_direction _rotvalue) (`Timeline|RotationDoor` :!label _label)
    (:`Update`
      (`SceneComponent.K2_SetRelativeRotation` (`self.RotPoint`) (`KismetMathLibrary.MakeRotator` (* _rotvalue (.roll (`self.RotationAxis`))) (* _rotvalue (.pitch (`self.RotationAxis`))) (* _rotvalue (.yaw (`self.RotationAxis`)))) false false))))

(event `UnRotate`
  (goto _label :!via `Reverse`))

(fn `Activate`
  (`parent.Activate`)
  (`self.Rotate`))

(fn `DeActivate`
  (`parent.DeActivate`)
  (if (`self.OpenClose?`)
    (`self.UnRotate`)))

(fn `UserConstructionScript`
  (`parent.UserConstructionScript`))