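; BP_P_PressurePlate is a pressure plate activator that responds only to a takable object of the required shape and size.
; When a BP_P_Takable overlaps its Box, it compares Shape and Scale against GoodShape and GoodSize.
; A match calls Activate on every actor in ActorToActivate, spawning FX_Activation at the Cube once per actor.
; When a matching object leaves, it calls DeActivate on those actors.
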(event `self.Box.OnComponentBeginOverlap`
  (params (OverlappedComponent :type "PrimitiveComponent Object Reference") (OtherActor :type "Actor Object Reference") (OtherComp :type "PrimitiveComponent Object Reference") (OtherBodyIndex :type Integer) (bFromSweep :type Boolean) (SweepResult :type "HitResult Structure (by ref)"))
  (bind _cube (`self.Cube`))
  (bind _asbp_p_takable (cast `/Game/Blueprints/Objects/BP_P_Takable` OtherActor))
  (if (`|EnumEquality` (`/Game/Blueprints/Objects/BP_P_Takable.Shape` _asbp_p_takable) (`self.GoodShape`))
    (if (`|EnumEquality` (`/Game/Blueprints/Objects/BP_P_Takable.Scale` _asbp_p_takable) (`self.GoodSize`))
      (for _array_element (`self.ActorToActivate`)
        (`/Game/Blueprints/GPE/Activable/BP_P_Activable.Activate` _array_element)
        (`KismetSystemLibrary.PrintString` "Activate")
        (`|SpawnActorFromClass` "/Game/VFX/2D/FX_Activation.FX_Activation_C" (`KismetMathLibrary.MakeTransform` (`SceneComponent.K2_GetComponentLocation` _cube) (`SceneComponent.K2_GetComponentRotation` _cube)) "Undefined" "OverrideRootScale" null null)))))

(event `self.Box.OnComponentEndOverlap`
  (params (OverlappedComponent :type "PrimitiveComponent Object Reference") (OtherActor :type "Actor Object Reference") (OtherComp :type "PrimitiveComponent Object Reference") (OtherBodyIndex :type Integer))
  (bind _asbp_p_takable (cast `/Game/Blueprints/Objects/BP_P_Takable` OtherActor))
  (if (`|EnumEquality` (`/Game/Blueprints/Objects/BP_P_Takable.Shape` _asbp_p_takable) (`self.GoodShape`))
    (if (`|EnumEquality` (`/Game/Blueprints/Objects/BP_P_Takable.Scale` _asbp_p_takable) (`self.GoodSize`))
      (for _array_element (`self.ActorToActivate`)
        (`/Game/Blueprints/GPE/Activable/BP_P_Activable.DeActivate` _array_element)))))

(fn `UserConstructionScript`)